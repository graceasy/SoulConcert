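; FloatingReadZone2 is an item actor that floats back and forth around its placed position, extending a parent class's behavior.
; On BeginPlay it runs the parent logic, stores the root component's world location, then starts a timeline.
; Each update teleport-free and sweep-free sets the actor location to that origin plus the timeline's Move offset.
; On finish, the timeline flips direction, creating an endless ping-pong loop without Tick.
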(event EventBeginPlay
  (|CallParentFunction)
  (bind _output_get (Variables|Components|SetInitial%20Position (Transformation|GetWorldLocation (Variables|Default|GetDefaultSceneRoot1))))
  (bind (_direction _move) (Timeline|Timeline_0 Play)
    (:Update
      (Transformation|SetActorLocation (+ _move _output_get) false false))
    (:Finished
      (switch Utilities|FlowControl|Switch|SwitchonETimelineDirection _direction
        (:Forward
          (Timeline|Timeline_0 ReverseFromEnd))
        (:Backward
          (Timeline|Timeline_0 PlayFromStart))))))

(event Collision|EventActorBeginOverlap
  (params (OtherActor :type Actor%20Object%20Reference))
  (|CallParentFunction OtherActor) ; 此节点被禁用，将不会被调用。\n从引脚连出引线来编译功能。
)

(event EventTick
  (params (DeltaSeconds :type Float%20%28single-precision%29))
  (|CallParentFunction DeltaSeconds) ; 此节点被禁用，将不会被调用。\n从引脚连出引线来编译功能。
)

(fn ConstructionScript
  (|CallParentFunction))