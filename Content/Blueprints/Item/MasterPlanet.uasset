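; MasterPlanet is a planet item actor, apparently a base for planets, that floats around its starting position while spinning.
; On BeginPlay it stores the static mesh's world location, then the Floating timeline adds its Move offset to that to set actor location.
; The timeline ping-pongs endlessly by reversing or replaying on finish.
; Tick adds a fixed yaw step each frame, unscaled by DeltaSeconds, so spin speed depends on frame rate.
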(event EventBeginPlay
  (|CallParentFunction)
  (bind _output_get (Variables|Default|SetInitial%20Position (Transformation|GetWorldLocation (Variables|Default|GetStaticMesh))))
  (bind (_direction _move) (Timeline|Floating Play)
    (:Update
      (Transformation|SetActorLocation (+ _move _output_get) false false))
    (:Finished
      (switch Utilities|FlowControl|Switch|SwitchonETimelineDirection _direction
        (:Forward
          (Timeline|Floating ReverseFromEnd))
        (:Backward
          (Timeline|Floating PlayFromStart))))))

(event EventTick
  (params (DeltaSeconds :type Float%20%28single-precision%29))
  (|CallParentFunction DeltaSeconds)
  (Class|Actor|AddActorWorldRotation (Math|Rotator|MakeRotator 0.0 0.0 (* 6e+01 0.003))))

(fn ConstructionScript
  (|CallParentFunction))