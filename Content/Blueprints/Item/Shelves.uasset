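; Shelves is an item actor with three mesh components that spin continuously.
; Each Tick adds a fixed local yaw to StaticMesh, Shelf2 and Shelf3 at different speeds, with Shelf2 turning slowly in the opposite direction.
; The increments ignore DeltaSeconds, so spin speed depends on frame rate.
; BeginPlay and the construction script only call their parents.
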(event EventBeginPlay
  (|CallParentFunction))

(event Collision|EventActorBeginOverlap
  (params (OtherActor :type Actor%20Object%20Reference))
  (|CallParentFunction OtherActor) ; 此节点被禁用，将不会被调用。\n从引脚连出引线来编译功能。
)

(event EventTick
  (params (DeltaSeconds :type Float%20%28single-precision%29))
  (|CallParentFunction DeltaSeconds)
  (Transformation|AddLocalRotation (Variables|Default|GetStaticMesh) (Math|Rotator|MakeRotator 0.0 0.0 (* 6e+01 0.002)) false false)
  (Transformation|AddLocalRotation (Variables|Default|Getshelf2) (Math|Rotator|MakeRotator 0.0 0.0 (* 6e+01 -0.0002)) false false)
  (Transformation|AddLocalRotation (Variables|Default|Getshelf3) (Math|Rotator|MakeRotator 0.0 0.0 (* 6e+01 0.003)) false false))

(fn ConstructionScript
  (|CallParentFunction))