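; Dog is a Blueprint actor that removes lightning notes it touches.
; Every tick it runs a short sphere trace on the Visibility channel from its skeletal mesh along the negative forward vector.
; A hit actor that casts to MasterNote and then LightningNote is destroyed, while other hits are ignored.
; Tick and the construction script both call the parent class, and nothing else is active.
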(event EventBeginPlay
  (|CallParentFunction) ; 此节点被禁用，将不会被调用。\n从引脚连出引线来编译功能。
)

(event Collision|EventActorBeginOverlap
  (params (OtherActor :type Actor%20Object%20Reference))
  (|CallParentFunction OtherActor) ; 此节点被禁用，将不会被调用。\n从引脚连出引线来编译功能。
)

(event EventTick
  (params (DeltaSeconds :type Float%20%28single-precision%29))
  (bind _skeletalmesh (Variables|Default|GetSkeletalMesh))
  (bind _returnvalue (Transformation|GetWorldLocation _skeletalmesh))
  (|CallParentFunction DeltaSeconds)
  (bind _outhit (Collision|SphereTraceByChannel _returnvalue (- _returnvalue (* (Math|Vector|GetForwardVector _skeletalmesh) 2e+01)) 2e+01 "TraceTypeQuery1" false 0 "None"))
  (bind _asmaster_note (Utilities|Casting|CastToMasterNote (.HitActor (Collision|BreakHitResult _outhit))))
  (bind _aslightning_note (Utilities|Casting|CastToLightningNote _asmaster_note))
  (Actor|DestroyActor _aslightning_note))

(fn ConstructionScript
  (|CallParentFunction))