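; MasterNPC is an NPC Blueprint with logic to move a static mesh along its spline, though nothing triggers that logic.
; Each Movement timeline update maps the Tracking value to a distance along the spline, then sets the mesh's world location and rotation and applies MoveRate as play rate.
; Location adds the local spline point to the root's world position, and local spline rotation serves as world rotation, so actor rotation is ignored.
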(fn ConstructionScript)